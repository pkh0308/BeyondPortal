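; BP_LaserEmitterd is a laser emitter actor that casts a beam reflecting off mirror surfaces.
; Tick, through a short Delay, calls CastLight from the Arrow component, which destroys and respawns all BP_LaserBeam segments each update.
; CastLight loops debug-drawn complex Visibility traces, mirroring direction by impact normal while the hit face's material is M_Mirror, with no bounce cap.
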(event `self.ReceiveTick`
  (params (DeltaSeconds :type "Float (single-precision)"))
  (bind _arrow (`self.Arrow`))
  (`KismetSystemLibrary.Delay` 0.01)
  (`self.CastLight` (`SceneComponent.K2_GetComponentLocation` _arrow) (`SceneComponent.GetForwardVector` _arrow) (`self.CastDIstance`)))

(fn `CastLight`
  (params (CastOrigin :type "Vector Structure") (CastDirection :type "Vector Structure") (CastDIstance :type "Float (double-precision)"))
  (locals (L_CastOrgin :type "Vector Structure") (L_CastDirection :type "Vector Structure") (L_CastDistace :type "Float (double-precision)") (L_Continue :type Boolean :default true) (L_BeamStart :type "Vector Structure") (L_BeamEnd :type "Vector Structure"))
  (bind _l_castorgin (`local.L_CastOrgin`))
  (bind _returnvalue (+ _l_castorgin (* (`local.L_CastDirection`) (`local.L_CastDistace`))))
  (set `local.L_CastOrgin` CastOrigin)
  (set `local.L_CastDirection` CastDirection)
  (set `local.L_CastDistace` CastDIstance)
  (for _array_element (`self.Beams`)
    (`self.K2_DestroyActor` _array_element))
  (`KismetArrayLibrary.Array_Clear` (`self.Beams`))
  (while (`local.L_Continue`)
    (`|ExecutionSequence`
      (:`then_0`
        (bind (_outhit _returnvalue_2) (`KismetSystemLibrary.LineTraceSingle` :`Start` _l_castorgin :`End` _returnvalue :`TraceChannel` "TraceTypeQuery1" :`bTraceComplex` true :`DrawDebugType` "ForDuration" :`DrawTime` 0.1))
        (set `local.L_BeamStart` (`local.L_CastOrgin`))
        (if _returnvalue_2
          (bind (_bblockinghit _binitialoverlap _time _distance _location _impactpoint _normal _impactnormal _physmat _hitactor _hitcomponent _hitbonename _bonename _hititem _elementindex _faceindex) (`GameplayStatics.BreakHitResult` _outhit))
          (set `local.L_BeamEnd` _impactpoint)
          (if (== (`.ReturnValue` (`PrimitiveComponent.GetMaterialFromCollisionFaceIndex` _hitcomponent _faceindex)) "/Game/SEB/Blueprints/Laser/M_Mirror.M_Mirror")
            (set `local.L_CastOrgin` _impactpoint)
            (set `local.L_CastDirection` (`KismetMathLibrary.MirrorVectorByNormal` (`local.L_CastDirection`) _impactnormal))
            (set `local.L_Continue` true)
            (else
              (set `local.L_Continue` false :!label _label)))
          (else
            (set `local.L_BeamEnd` _returnvalue)
            (goto _label))))
      (:`then_1`
        (bind _returnvalue_3 (`|SpawnActorFromClass` "/Game/SEB/Blueprints/Laser/BP_LaserBeam.BP_LaserBeam_C" (`KismetMathLibrary.MakeTransform` (0.0 0.0 0.0)) "Undefined" "MultiplyWithRoot" null null))
        (`/Game/SEB/Blueprints/Laser/BP_LaserBeam.SetEnds` _returnvalue_3 (`local.L_BeamStart`) (`local.L_BeamEnd`))
        (`KismetArrayLibrary.Array_Add` (`self.Beams`) _returnvalue_3)))))

(fn `UserConstructionScript`)