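; Laser emitter actor that casts a red beam from its Arrow, bouncing off mirrors and relaying through sensors.
; Tick, behind a short Delay, calls CastLight, which loops line traces and reflects on M_Mirror, flattening bounces with low Z.
; M_SensorMaterial hits recursively recast from that actor's forward vector.
; Each cast updates one Niagara beam and respawns BP_LaserBeam segments, whose endpoint variables are never assigned here.
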(event `self.ReceiveBeginPlay`
  (`FXSystemComponent.SetColorParameter` (`self.NiagaraLaser`) "Color" (struct :`R` 1.0 :`A` 1.0)))

(event `self.ReceiveTick`
  (params (DeltaSeconds :type "Float (single-precision)"))
  (bind _arrow (`self.Arrow`))
  (`KismetSystemLibrary.Delay` 0.01)
  (`self.CastLight` (`SceneComponent.K2_GetComponentLocation` _arrow) (`SceneComponent.GetForwardVector` _arrow) 1000.0))

(fn `CastLight`
  (params (CastOrigin :type "Vector Structure") (CastDirection :type "Vector Structure") (CastDistance :type "Float (double-precision)"))
  (locals (L_CastOrigin :type "Vector Structure") (L_CastDirection :type "Vector Structure") (L_CastDistance :type "Float (double-precision)") (L_Continue :type Boolean :default true) (L_BeamStart :type "Vector Structure") (L_BeamEnd :type "Vector Structure"))
  (bind _returnvalue (+ (`local.L_CastOrigin`) (* (`local.L_CastDirection`) (`local.L_CastDistance`))))
  (set `local.L_CastOrigin` CastOrigin)
  (set `local.L_CastDirection` CastDirection)
  (set `local.L_CastDistance` CastDistance)
  (`FXSystemComponent.SetVectorParameter` (`self.NiagaraLaser`) "LaserStart" (`local.L_CastOrigin`))
  (bind _output_get (set `self.TraceEnd` _returnvalue))
  (`FXSystemComponent.SetVectorParameter` (`self.NiagaraLaser`) "LaserEnd" _output_get)
  (for _array_element (`self.Beams`)
    (`self.K2_DestroyActor` _array_element))
  (`KismetArrayLibrary.Array_Clear` (`self.Beams`))
  (while (`local.L_Continue`)
    (`|ExecutionSequence`
      (:`then_0`
        (bind (_outhit _returnvalue_2) (`KismetSystemLibrary.LineTraceSingle` :`Start` (`local.L_CastOrigin`) :`End` _returnvalue :`TraceChannel` "TraceTypeQuery1" :`DrawDebugType` "ForOneFrame" :`TraceColor` (struct :`R` 1.0) :`TraceHitColor` (struct :`G` 1.0)))
        (`FXSystemComponent.SetVectorParameter` (`self.NiagaraLaser`) "LaserStart" (`local.L_CastOrigin`))
        (if _returnvalue_2
          (bind (_bblockinghit _binitialoverlap _time _distance _location _impactpoint _normal _impactnormal _physmat _hitactor _hitcomponent _hitbonename _bonename _hititem _elementindex _faceindex) (`GameplayStatics.BreakHitResult` _outhit))
          (`FXSystemComponent.SetVectorParameter` (`self.NiagaraLaser`) "LaserEnd" _impactpoint)
          (bind (_sectionindex _returnvalue_3) (`PrimitiveComponent.GetMaterialFromCollisionFaceIndex` _hitcomponent _faceindex))
          (if (== _returnvalue_3 "/Game/SEB/Blueprints/Laser/M_Mirror.M_Mirror")
            (set `local.L_CastOrigin` _impactpoint)
            (bind (_returnvalue_x _returnvalue_y _returnvalue_z) (`KismetMathLibrary.BreakVector` (`KismetMathLibrary.MirrorVectorByNormal` (`local.L_CastDirection`) _impactnormal)))
            (if (<= _returnvalue_z 0.5)
              (set `local.L_CastDirection` (`KismetMathLibrary.MakeVector` _returnvalue_x _returnvalue_y))
              (else
                (set `local.L_CastDirection` (`KismetMathLibrary.MakeVector` _returnvalue_x _returnvalue_y _returnvalue_z))))
            (set `local.L_Continue` true)
            (else
              (if (== _returnvalue_3 "/Game/SEB/Blueprints/Laser/M_SensorMaterial.M_SensorMaterial")
                (`self.CastLight` (`self.K2_GetActorLocation` _hitactor) (`self.GetActorForwardVector` _hitactor) (`local.L_CastDistance`)))
              (set `local.L_Continue` false)))
          (else
            (`FXSystemComponent.SetVectorParameter` (`self.NiagaraLaser`) "LaserEnd" (`self.TraceEnd`)))))
      (:`then_1`
        (bind _returnvalue_4 (`|SpawnActorFromClass` "/Game/SEB/Blueprints/Laser/BP_LaserBeam.BP_LaserBeam_C" (`KismetMathLibrary.MakeTransform` (0.0 0.0 0.0)) "Undefined" "MultiplyWithRoot" null null))
        (`/Game/SEB/Blueprints/Laser/BP_LaserBeam.SetEnds` _returnvalue_4 (`local.L_BeamStart`) (`local.L_BeamEnd`))
        (`KismetArrayLibrary.Array_Add` (`self.Beams`) _returnvalue_4)))))

(fn `UserConstructionScript`)